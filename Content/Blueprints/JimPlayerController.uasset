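; JimPlayerController handles the player character's facing direction and the background music.
; BeginPlay finds the first JimCharacter and sets its starting rotation, then ChangePlayerRotation uses a FlipFlop to alternate it between left and right rotations.
; Two audio finished events hand playback back and forth between Music and Music1 as a loop.
; Pressing E sharply raises the pitch multiplier on Music only, to speed it up.
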(event Custom|OnAudioFinished_Event2
  (bind _music (Variables|Default|GetMusic))
  ;[1 1 1] Set Music
  (Audio|Components|Audio|Play _music 0.0)
  (EventDispatchers|BindEventtoOnAudioFinished _music (delegate Custom|OnAudioFinished_Event)))

(event Custom|ChangePlayerRotation
  ;[1 1 1] Changes Direction of Player
  (Utilities|FlowControl|FlipFlop
    (:A
      (Transformation|SetActorRotation (stale EventBeginPlay _asjim_character) (Variables|Default|GetLeftDirectionPawn)))
    (:B
      (Transformation|SetActorRotation (stale EventBeginPlay _asjim_character) (Variables|Default|GetRightDirectionPawn)))))

(event Custom|OnAudioFinished_Event
  (bind _music1 (Variables|Default|GetMusic1))
  ;[1 1 1] Set Music
  (Audio|Components|Audio|Play _music1 0.0)
  (EventDispatchers|BindEventtoOnAudioFinished _music1 (delegate Custom|OnAudioFinished_Event2)))

(event EventBeginPlay
  ;[1 1 1] Set Direction of Player at Game Start
  (bind _outactors (Actor|GetAllActorsOfClass "/Game/Blueprints/JimCharacter.JimCharacter_C"))
  (Variables|Default|Setstored (Utilities|Array|Get(acopy) _outactors))
  (bind _asjim_character (Utilities|Casting|CastToJimCharacter (Variables|Default|Getstored)))
  (Transformation|SetActorRotation _asjim_character "0.000000,-90.000000, 0"))

(event Input|KeyboardEvents|E
  (params (Key :type Key%20Structure :default "AnyKey"))
  ;[1 1 1] Change Music Speed
  (:Pressed
    (Audio|Components|Audio|SetPitchMultiplier (Variables|Default|GetMusic) 12.0)))

(fn ConstructionScript)