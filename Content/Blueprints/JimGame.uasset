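; JimGame controls the game flow for Jim: starting a run, ending it on death and restarting the level via console command.
; Starting enables character and level-item movement and runs a delay loop that steadily raises the score on JimHUD.
; Death stops movement, saves any new high score to the "JIM" save slot and shows the game-over menu.
; BeginPlay loads the saved high score and caches the HUD.
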(event Custom|SaveScore
  (bind _score (Variables|Default|GetScore))
  ;[1 1 1] Save Game
  (if (> (Variables|Default|GetScore) (Variables|Default|GetHighScore))
    (Variables|Default|SetHighScore (Variables|Default|GetScore))
    (bind _returnvalue (SaveGame|DoesSaveGameExist "JIM"))
    (if _returnvalue
      (bind _asjim_save_game (Utilities|Casting|CastToJimSaveGame (Variables|Default|GetSaveGameObject)))
      (Variables|/Game/Blueprints/JimSaveGame.JimSaveGame_C|SetSavedHighScore _asjim_save_game _score)
      (SaveGame|SaveGametoSlot (Variables|Default|GetSaveGameObject) "JIM")
      (Development|PrintString "saved" true true "(R=1.000000,G=0.000000,B=0.958813,A=1.000000)")
      (else
        (bind _returnvalue_2 (SaveGame|CreateSaveGameObject "/Game/Blueprints/JimSaveGame.JimSaveGame_C"))
        (Variables|Default|SetSaveGameObject _returnvalue_2)
        (bind _asjim_save_game_2 (Utilities|Casting|CastToJimSaveGame (Variables|Default|GetSaveGameObject)))
        (Variables|/Game/Blueprints/JimSaveGame.JimSaveGame_C|SetSavedHighScore _asjim_save_game_2 _score)
        (SaveGame|SaveGametoSlot (Variables|Default|GetSaveGameObject) "JIM")
        (Development|PrintString "MADE NEW SAVE GAME" true true "(R=1.000000,G=0.000000,B=0.958813,A=1.000000)")))))

(event Custom|JimDead
  (bind _jimhud (Variables|Default|GetJimHUD))
  ;[1 1 1] Jim Dies, turn off movement and turn on new hud
  (Variables|/Game/Blueprints/JimCharacter.JimCharacter_C|Setcanmove (Variables|Default|GetJimPC) false)
  (Variables|Default|Setcanmovelevelitems false)
  (CallFunction|SaveScore)
  (Variables|/Game/Blueprints/JimHUD.JimHUD_C|SetDrawGameOver _jimhud true)
  (Variables|/Game/Blueprints/JimHUD.JimHUD_C|SetDrawMenu _jimhud true))

(event Custom|StartJimGame
  ;[1 1 1] Start game and enable movement
  (bind _outactors (Actor|GetAllActorsOfClass "/Game/Blueprints/JimCharacter.JimCharacter_C"))
  (Variables|Default|SetActor (Utilities|Array|Get(acopy) _outactors))
  (bind _asjim_character (Utilities|Casting|CastToJimCharacter (Variables|Default|GetActor)))
  (Variables|Default|SetJimPC _asjim_character)
  (Variables|/Game/Blueprints/JimCharacter.JimCharacter_C|Setcanmove (Variables|Default|GetJimPC) true)
  (Variables|Default|Setcanmovelevelitems true)
  ;[1 1 1] Increment Score and Set HUD Score
  (if (Variables|Default|Getcanmovelevelitems) :!label _label
    (Variables|Default|SetScore (+ (Variables|Default|GetScore) 1))
    (Utilities|FlowControl|Delay 0.1)
    (Variables|/Game/Blueprints/JimHUD.JimHUD_C|SetCurrentScore (Variables|Default|GetJimHUD) (Variables|Default|GetScore))
    (goto _label)))

(event Custom|ResetGame
  ;[1 1 1] Restart Level / Game
  (Development|ExecuteConsoleCommand "restartlevel" (Game|GetPlayerController 0)))

(event EventBeginPlay
  ;[1 1 1] Get Players hud and load save game if there is one
  (bind _returnvalue (SaveGame|DoesSaveGameExist "JIM"))
  (if _returnvalue
    (bind _returnvalue_2 (SaveGame|LoadGamefromSlot "JIM"))
    (Variables|Default|SetSaveGameObject _returnvalue_2)
    (bind _asjim_save_game (Utilities|Casting|CastToJimSaveGame (Variables|Default|GetSaveGameObject)))
    (Variables|Default|SetHighScore (Variables|/Game/Blueprints/JimSaveGame.JimSaveGame_C|GetSavedHighScore _asjim_save_game))
    (CallFunction|SetupHUD)
    (else
      (CallFunction|SetupHUD))))

(fn ConstructionScript)

(fn SetupHUD
  (bind _asjim_hud (Utilities|Casting|CastToJimHUD (HUD|GetHUD (Game|GetPlayerController 0))))
  (Variables|Default|SetJimHUD _asjim_hud))