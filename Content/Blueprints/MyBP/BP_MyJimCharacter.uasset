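; Player character Blueprint for Jim that handles his death and the level restart that follows.
; JimDie runs once, calls the parent version, disables camera movement and control, and plays the death animation and sound.
; After short delays it sets the game-start flag on BP_JimCppGameMode, hides the mesh and destroys the actor.
; The Destroyed event restarts the level through the RestartLevel console command.
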(event EventDestroyed
  (Development|ExecuteConsoleCommand "RestartLevel"))

(event EventJimDie
  ;[1 0.3199 0.28] Die
  (Utilities|FlowControl|DoOnce false
    (:Completed
      (|CallParentFunction)
      (Variables|Default|SetShouldMoveCamera false)
      (Variables|Default|SetbCanMove false)
      (Components|Animation|PlayAnimation (Variables|Character|GetMesh) "/Game/JimCharacter/Anim_Jim_DeathAbove.Anim_Jim_DeathAbove" false)
      (Audio|PlaySound2D "/Game/Audio/JimDeath.JimDeath")
      (Utilities|FlowControl|Delay 0.8)
      (Class|JimCppGameMode|SetIsGameStart (.AsBP%20Jim%20Cpp%20Game%20Mode (Utilities|Casting|CastToBP_JimCppGameMode (Game|GetGameMode))) true)
      (Rendering|SetVisibility (Variables|Character|GetMesh) false false)
      (Utilities|FlowControl|Delay 3.0)
      (Actor|DestroyActor))))

(fn ConstructionScript)