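; JimHUD is the game's canvas HUD, drawing the start menu, the in-play score and the game-over screen with final and high scores.
; DrawHUD switches screens on two flags, drawing buttons and art as regions of one texture atlas with hit boxes over the buttons.
; Button clicks play a sound and call the JimGame game mode, cached on BeginPlay, to start or, after a short delay, reset the game.
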(event Custom|DrawScore
  ;[1 1 1] DrawScore
  (HUD|DrawText "SCORE" "(R=1.000000,G=1.000000,B=1.000000,A=1.000000)" (- (* (Variables|Default|GetScreenSizeX) 0.5) 75.0) 25.0 "/Game/DontDropJimAssets/JimFont.JimFont" 1.0 false)
  (HUD|DrawText (Utilities|String|ToString(Integer) (Variables|Default|GetCurrentScore)) "(R=1.000000,G=1.000000,B=1.000000,A=1.000000)" (+ (* (Variables|Default|GetScreenSizeX) 0.5) 55.0) 25.0 "/Game/DontDropJimAssets/JimFont.JimFont" 1.0 false))

(event Custom|DrawFinalScore
  ;[1 1 1] Draw Final Score and High Score
  (HUD|DrawText (Utilities|String|ToString(Integer) (Variables|/Game/Blueprints/JimGame.JimGame_C|GetHighScore (Variables|Default|GetJimGameStore))) "(R=1.000000,G=1.000000,B=1.000000,A=1.000000)" (- (* (Variables|Default|GetScreenSizeX) 0.5) -35.0) 125.0 "/Game/DontDropJimAssets/JimFont.JimFont" 1.0 false)
  (HUD|DrawText (Utilities|String|ToString(Integer) (Variables|Default|GetCurrentScore)) "(R=1.000000,G=1.000000,B=1.000000,A=1.000000)" (- (* (Variables|Default|GetScreenSizeX) 0.5) -35.0) 65.0 "/Game/DontDropJimAssets/JimFont.JimFont" 1.0 false))

(event EventDrawHUD
  (params (SizeX :type Integer) (SizeY :type Integer))
  ;[1 1 1] Draw Start Menu
  (Variables|Default|SetScreenSizeX SizeX)
  (Variables|Default|SetScreenSizeY SizeY)
  (if (Variables|Default|GetDrawMenu)
    (if (Variables|Default|GetDrawGameOver)
      ;[1 1 1] Draw End Menu
      (Canvas|DrawTexture (Variables|Default|GetPlayTexture) (- (* (Variables|Default|GetScreenSizeX) 0.5) (* (Variables|Default|GetResetXSize) 0.5)) (Variables|Default|GetResetYPos) (Variables|Default|GetResetXSize) (Variables|Default|GetResetYSize) 0.604 0.012 0.19 0.197 "(R=1.000000,G=1.000000,B=1.000000,A=1.000000)" "BLEND_Masked")
      (Class|HUD|AddHitBox (Math|Vector2D|MakeVector2D (- (* (Variables|Default|GetScreenSizeX) 0.5) (* (Variables|Default|GetResetXSize) 0.5)) (Variables|Default|GetResetYPos)) (Math|Vector2D|MakeVector2D (Variables|Default|GetResetXSize) (Variables|Default|GetResetYSize)) "None" false)
      (Canvas|DrawTexture (Variables|Default|GetPlayTexture) (- (* (Variables|Default|GetScreenSizeX) 0.5) (* (Variables|Default|GetGameOverXSize) 0.5)) (Variables|Default|GetGameOverYPos) (Variables|Default|GetGameOverXSize) (Variables|Default|GetGameOverYSize) 0.222 0.389 0.565 0.23 "(R=1.000000,G=1.000000,B=1.000000,A=1.000000)" "BLEND_Masked")
      (CallFunction|DrawFinalScore)
      (else
        (Canvas|DrawTexture (Variables|Default|GetPlayTexture) (- (* (Variables|Default|GetScreenSizeX) 0.5) (* (Variables|Default|GetPlayXSize) 0.5)) (Variables|Default|GetPlayYPos) (Variables|Default|GetPlayXSize) (Variables|Default|GetPlayYSize) 0.0147 0.238 0.2 0.197 "(R=1.000000,G=1.000000,B=1.000000,A=1.000000)" "BLEND_Masked")
        (Class|HUD|AddHitBox (Math|Vector2D|MakeVector2D (- (* (Variables|Default|GetScreenSizeX) 0.5) (* (Variables|Default|GetPlayXSize) 0.5)) (Variables|Default|GetPlayYPos)) (Math|Vector2D|MakeVector2D (Variables|Default|GetPlayXSize) (Variables|Default|GetPlayYSize)) (Variables|Default|GetPlayBox) false 1)
        (Canvas|DrawTexture (Variables|Default|GetPlayTexture) (- (* (Variables|Default|GetScreenSizeX) 0.5) (* (Variables|Default|GetLogoXSize) 0.5)) (Variables|Default|GetLogoYSize) (Variables|Default|GetLogoXPos) (Variables|Default|GetLogoYPos) 0.006 0.003 0.572 0.226 "(R=1.000000,G=1.000000,B=1.000000,A=1.000000)" "BLEND_Masked")))
    (else
      (CallFunction|DrawScore))))

(event EventBeginPlay
  ;[1 1 1] Grab game mode, turn off end menu just in case, set up ygap to add to position to help spacing
  (Variables|Default|SetDrawGameOver false)
  (Variables|Default|SetPlayYPos (+ (Variables|Default|GetPlayYPos) (Variables|Default|GetYGAP)))
  (bind _asjim_game (Utilities|Casting|CastToJimGame (Game|GetGameMode)))
  (Variables|Default|SetJimGameStore _asjim_game))

(event EventHitBoxClick
  (params (BoxName :type Name :default "None"))
  ;[1 1 1] If we've clicked a button check which one, then either start / reset game
  (if (Utilities|Name|Equal(Name) BoxName (Variables|Default|GetPlayBox))
    (Variables|Default|SetDrawMenu false)
    (Default|StartJimGame (Variables|Default|GetJimGameStore))
    (Audio|Components|Audio|Play (Variables|Default|GetButtonClickCue) 0.0)
    (elif (Utilities|Name|Equal(Name) BoxName (Variables|Default|GetResetBox))
      (Variables|Default|SetDrawGameOver false)
      (Audio|Components|Audio|Play (Variables|Default|GetButtonClickCue) 0.0)
      (Utilities|FlowControl|Delay 0.2)
      (Default|ResetGame (Variables|Default|GetJimGameStore)))))

(fn ConstructionScript)